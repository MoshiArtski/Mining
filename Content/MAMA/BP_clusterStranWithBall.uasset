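; Chaos field system Blueprint that launches a ball and applies cluster strain to break geometry collections within a box.
; Toggle waits briefly, then applies a box-culled integer field that switches objects inside the box from kinematic to dynamic.
; It then multiplies a uniform direction vector by a radial falloff at the Sphere to apply linear velocity only there.
; Finally, a box falloff applies external cluster strain throughout the same box.
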(event EventToggle
  (params (On/off :type Boolean))
  (Utilities|FlowControl|Delay 1.0)
  ;[0.2702 1 0.9701] Using a box falloff as a culling field to switch the ball from kinematic to dynamic
  (Class|FieldSystemComponent|ApplyPhysicsField (Variables|Field|GetFieldSystemComponent) true "Field_DynamicState" 0 (Field|SetCullingField (Variables|Default|GetCullingField) (Field|SetBoxFalloff (Variables|Default|GetBoxFalloff) 1.0 0.0 1.0 0.0 (Transformation|GetWorldTransform (Variables|Default|GetBox)) "Field_FallOff_None") (Field|SetUniformInteger (Variables|Default|GetUniformInteger) (Math|Conversions|ToInteger(Byte) (Variables|Default|GetDynamic))) "Field_Culling_Outside"))
  ;[0.1749 0.3953 1] Apply force to the Ball
  (Class|FieldSystemComponent|ApplyPhysicsField (Variables|Field|GetFieldSystemComponent) true "Field_LinearVelocity" 0 (Field|SetOperatorField (Variables|Default|GetOperatorField) (Variables|Default|GetforceMagnitude) (Field|SetUniformVector (Variables|Default|GetUniformVector) 1.0 (Variables|Default|Getdirection)) (Field|SetRadialFalloff (Variables|Default|GetRadialFalloff) 1.0 0.0 1.0 0.0 1e+02 (Transformation|GetWorldLocation (Variables|Default|GetSphere)) "Field_FallOff_None") "Field_Multiply"))
  ;[0.2257 1 0.2706] Apply Physics Field nodes determine what attributes are affected by your field
  (Class|FieldSystemComponent|ApplyPhysicsField (Variables|Field|GetFieldSystemComponent) true "Field_ExternalClusterStrain" 0 (Field|SetBoxFalloff (Variables|Default|GetBoxFalloff) (Variables|Default|Getmagnitude) 0.0 1.0 0.0 (Transformation|GetWorldTransform (Variables|Default|GetBox)) "Field_FallOff_None")))

(event EventBeginPlay)

(event EventTick
  (params (DeltaSeconds :type Float%20%28single-precision%29)))

(fn ConstructionScript)