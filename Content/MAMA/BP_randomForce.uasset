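; Field system actor that breaks up Geometry Collections and scatters the pieces with randomly moving physics fields.
; CallTriggerActor enables cluster strain, then applies it with a radial linear force and random torque, all sized by SphereCol.
; Tick uses a Delay to re-randomize the X/Z offset every half second and re-apply the fields.
; Only strain honors the Enabled flag; force and torque apply even before triggering.
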(event EventTick
  (params (DeltaSeconds :type Float%20%28single-precision%29))
  (bind _fieldsystemcomponent (Variables|Field|GetFieldSystemComponent))
  (bind _spherecol (Variables|Default|GetSphereCol))
  (bind _spherecol_2 (Variables|Default|GetSphereCol))
  (bind _returnvalue (Transformation|GetWorldLocation _spherecol))
  (bind _returnvalue_2 (Transformation|GetWorldLocation _spherecol_2))
  ;[0 0.1382 1 0.25] Force Field
  (Utilities|FlowControl|Delay 0.5)
  ;;[0.07741 0.8108 0 0.25] Randomize the field's x and z position over time.
  (Variables|Default|SetxValue (* (- (* (Math|Random|RandomFloat) 2.0) 1.0) 2e+02))
  (Variables|Default|SetzValue (* (- (* (Math|Random|RandomFloat) 2.0) 1.0) 2e+02))
  ;;[0.5295 0.04161 0.201 0.25] Apply strain to break up clustered geometry collection.
  (Class|FieldSystemComponent|ApplyPhysicsField _fieldsystemcomponent (stale EventCallTriggerActor _output_get) "Field_ExternalClusterStrain" 0 (Field|SetRadialFalloff (Variables|Default|GetRadialFalloff%20-%20Strain) (Variables|Default|GetstrainMagnitude) 0.0 1.0 0.0 (Components|Sphere|GetScaledSphereRadius _spherecol_2) (+ (Math|Vector|MakeVector (+ (Variables|Default|GetxValue) (.x _returnvalue_2)) (.y _returnvalue_2) (+ (.z _returnvalue_2) (Variables|Default|GetzValue))) "0, 0, 0") "Field_FallOff_None"))
  ;;[0 0.1382 1 0.25] Force
  (Class|FieldSystemComponent|ApplyPhysicsField _fieldsystemcomponent true "Field_LinearForce" 0 (Field|SetOperatorField (Variables|Default|GetOperatorField%20-%20Force) 1.0 (Field|SetRadialVector (Variables|Default|GetRadialVector%20-%20Force) (Variables|Default|GetforceMagnitude) (+ (Math|Vector|MakeVector (+ (Variables|Default|GetxValue) (.x _returnvalue)) (.y _returnvalue) (+ (.z _returnvalue) (Variables|Default|GetzValue))) "0, 0, 0")) (Field|SetRadialFalloff (Variables|Default|GetRadialFalloff%20-%20Force) 1.0 0.0 1.0 0.0 (Components|Sphere|GetScaledSphereRadius _spherecol) (+ (Math|Vector|MakeVector (+ (Variables|Default|GetxValue) (.x _returnvalue)) (.y _returnvalue) (+ (.z _returnvalue) (Variables|Default|GetzValue))) "0, 0, 0") "Field_Falloff_Linear") "Field_Multiply"))
  (Class|FieldSystemComponent|ApplyPhysicsField _fieldsystemcomponent true "Field_AngularTorque" 0 (Field|SetOperatorField (Variables|Default|GetOperatorField%20-%20Torque) 1.0 (Field|SetRadialFalloff (Variables|Default|GetRadialFalloff%20-%20Force) 1.0 0.0 1.0 0.0 (Components|Sphere|GetScaledSphereRadius _spherecol) (+ (Math|Vector|MakeVector (+ (Variables|Default|GetxValue) (.x _returnvalue)) (.y _returnvalue) (+ (.z _returnvalue) (Variables|Default|GetzValue))) "0, 0, 0") "Field_Falloff_Linear") (Class|RandomVector|SetRandomVector (Variables|Default|GetRandomVector%20-%20Torque) 1.0) "Field_Multiply")))

(event EventCallTriggerActor
  (bind _fieldsystemcomponent (Variables|Field|GetFieldSystemComponent))
  (bind _radialfalloff___force (Variables|Default|GetRadialFalloff%20-%20Force))
  (bind _xvalue (Variables|Default|GetxValue))
  (bind _zvalue (Variables|Default|GetzValue))
  (bind _spherecol (Variables|Default|GetSphereCol))
  (bind _spherecol_2 (Variables|Default|GetSphereCol))
  (bind _returnvalue (Transformation|GetWorldLocation _spherecol))
  (bind _returnvalue_2 (Components|Sphere|GetScaledSphereRadius _spherecol))
  (bind _returnvalue_3 (Transformation|GetWorldLocation _spherecol_2))
  (bind _returnvalue_4 (+ (.z _returnvalue) _zvalue))
  (bind _returnvalue_5 (+ _xvalue (.x _returnvalue)))
  (bind _returnvalue_6 (+ (Math|Vector|MakeVector _returnvalue_5 (.y _returnvalue) _returnvalue_4) "0, 0, 0"))
  (bind _returnvalue_7 (Field|SetRadialFalloff _radialfalloff___force 1.0 0.0 1.0 0.0 _returnvalue_2 _returnvalue_6 "Field_Falloff_Linear"))
  ;[0 0.1382 1 0.25] Force Field
  ;;[0.5295 0.04161 0.201 0.25] Apply strain to break up clustered geometry collection.
  (bind _output_get (Variables|Default|SetEnabled true))
  (Class|FieldSystemComponent|ApplyPhysicsField _fieldsystemcomponent _output_get "Field_ExternalClusterStrain" 0 (Field|SetRadialFalloff (Variables|Default|GetRadialFalloff%20-%20Strain) (Variables|Default|GetstrainMagnitude) 0.0 1.0 0.0 (Components|Sphere|GetScaledSphereRadius _spherecol_2) (+ (Math|Vector|MakeVector (+ (Variables|Default|GetxValue) (.x _returnvalue_3)) (.y _returnvalue_3) (+ (.z _returnvalue_3) (Variables|Default|GetzValue))) "0, 0, 0") "Field_FallOff_None"))
  ;;[0 0.1382 1 0.25] Force
  (Class|FieldSystemComponent|ApplyPhysicsField _fieldsystemcomponent true "Field_LinearForce" 0 (Field|SetOperatorField (Variables|Default|GetOperatorField%20-%20Force) 1.0 (Field|SetRadialVector (Variables|Default|GetRadialVector%20-%20Force) (Variables|Default|GetforceMagnitude) _returnvalue_6) _returnvalue_7 "Field_Multiply"))
  (Class|FieldSystemComponent|ApplyPhysicsField _fieldsystemcomponent true "Field_AngularTorque" 0 (Field|SetOperatorField (Variables|Default|GetOperatorField%20-%20Torque) 1.0 _returnvalue_7 (Class|RandomVector|SetRandomVector (Variables|Default|GetRandomVector%20-%20Torque) 1.0) "Field_Multiply")))

(fn ConstructionScript)