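; BP_NoiseField is a Chaos field actor that, when triggered, breaks up geometry collections inside its box and pushes and spins the pieces.
; After a short delay it applies box-falloff external cluster strain to release clustered pieces.
; It then applies a linear force from a noise field multiplied by a uniform vector, and angular torque from a scaled random vector.
; Culling fields confine both force and torque to the box volume.
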(event EventCallTriggerActor
  (bind _box (Variables|Default|GetBox))
  (bind _boxfalloff_culling (Variables|Default|GetBoxFalloff_culling))
  (bind _returnvalue (Transformation|GetWorldTransform _box))
  (bind _returnvalue_2 (Field|SetBoxFalloff _boxfalloff_culling 1.0 0.0 1.0 0.0 _returnvalue "Field_FallOff_None"))
  (Utilities|FlowControl|Delay 0.15)
  ;[1 0.1231 0.09321] Apply strain to break up clustered geometry collection before forces can be applied
  (Class|FieldSystemComponent|ApplyPhysicsField (Variables|Field|GetFieldSystemComponent) true "Field_ExternalClusterStrain" 0 (Field|SetBoxFalloff (Variables|Default|GetBoxFalloff_strain) (Variables|Default|GetstrainMagnitude) 0.0 1.0 0.0 (Transformation|GetWorldTransform (Variables|Default|GetBox)) "Field_FallOff_None"))
  ;[0.8307 0 1] Force
  ;;[1 1 1] Scalar Multiplier for Noise Field
  (bind _output_get (Variables|Default|SettransformVar (Transformation|GetWorldTransform (Variables|Default|GetBox))))
  (Class|FieldSystemComponent|ApplyPhysicsField (Variables|Field|GetFieldSystemComponent) true "Field_LinearForce" 0 (Field|SetCullingField (Variables|Default|GetCullingField_force) _returnvalue_2 (Field|SetOperatorField (Variables|Default|GetOperatorField_noise) 1.0 (Class|NoiseField|SetNoiseField (Variables|Default|GetNoiseField) -1.0 1.0 (Math|Transform|MakeTransform "0, 0, 0" "0, 0, 0" (* (.scale _output_get) (Variables|Default|GetnoiseScale)))) (Field|SetUniformVector (Variables|Default|GetUniformVector_force) (Variables|Default|GetforceMagnitude) "0.000000,2.000000,0.000000") "Field_Multiply") "Field_Culling_Outside"))
  ;[0 0.1279 1] Rotation
  (Class|FieldSystemComponent|ApplyPhysicsField (Variables|Field|GetFieldSystemComponent) true "Field_AngularTorque" 0 (Field|SetCullingField (Variables|Default|GetCullingField_rotation) _returnvalue_2 (Field|SetOperatorField (Variables|Default|GetOperatorField_rotation) 1.0 (Class|RandomVector|SetRandomVector (Variables|Default|GetRandomVector) (Variables|Default|GetrotationMagnitude)) (Field|SetUniformVector (Variables|Default|GetUniformVector_rotation) 1.0 (Variables|Default|GetrotationMult)) "Field_Multiply") "Field_Culling_Outside")))

(fn ConstructionScript)